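; EnemyPaddle_BP is the computer-controlled opponent paddle, which slides along the Y axis to track the InvisibleBall_BP actor rather than a visible ball.
; Each Tick looks up that actor by class, stores its location as the target, and calls SetDirection to choose the sign of movement.
; The paddle then moves by a fixed per-frame step, unscaled by delta time, and is snapped back inside hard-coded Y limits.
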(event EventBeginPlay)

(event Collision|EventActorBeginOverlap
  (params (OtherActor :type Actor%20Object%20Reference)))

(event EventTick
  (params (DeltaSeconds :type Float%20%28single-precision%29))
  (bind _returnvalue (Transformation|GetActorLocation))
  (bind _returnvalue_2 (Transformation|GetActorLocation))
  (bind _returnvalue_3 (Transformation|GetActorLocation))
  (bind (_x _y _z) (Math|Vector|BreakVector _returnvalue))
  (bind (_x_2 _y_2 _z_2) (Math|Vector|BreakVector _returnvalue_2))
  (bind _y_3 (Math|Vector|BreakVector _returnvalue_3))
  (bind _returnvalue_4 (Actor|GetActorOfClass "/Game/InvisibleBall_BP.InvisibleBall_BP_C"))
  (Variables|Default|SettargetPosition (Transformation|GetActorLocation _returnvalue_4))
  (CallFunction|SetDirection)
  (Transformation|AddActorLocalOffset (Math|Vector|MakeVector 0.0 (* (Variables|Default|GetmoveDir) (Variables|Default|GetmoveSpeed)) 0.0) false false)
  (if (< _y_3 -4.7e+02)
    (Transformation|SetActorLocation (Math|Vector|MakeVector _x_2 -469.0 _z_2) false false)
    (elif (> _y_3 4.7e+02)
      (Transformation|SetActorLocation (Math|Vector|MakeVector _x 469.0 _z) false false))))

(fn ConstructionScript)

(fn SetDirection
  (if (<= (.Y (Math|Vector|BreakVector (Transformation|GetActorLocation))) (.Y (Math|Vector|BreakVector (Variables|Default|GettargetPosition))))
    (Variables|Default|SetmoveDir 1)
    (elif (>= (.Y (Math|Vector|BreakVector (Transformation|GetActorLocation))) (.Y (Math|Vector|BreakVector (Variables|Default|GettargetPosition))))
      (Variables|Default|SetmoveDir -1)
      (else
        (Variables|Default|SetmoveDir 0)))))