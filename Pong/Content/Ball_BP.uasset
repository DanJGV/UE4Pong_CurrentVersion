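; Pong-style ball that bounces between a player paddle and an enemy paddle via ProjectileMovement velocity.
; Paddle hits reverse X with randomized spin based on paddle movement and speed up X, while walls reverse Y.
; Tagged player paddle hits also move InvisibleBall_BP to the ball and trigger its CopyVelocity before the speed-up.
; Tick resets the ball to the origin with a fixed velocity once it passes either paddle's X position.
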(event Collision|EventActorBeginOverlap
  (params (OtherActor :type Actor%20Object%20Reference))
  (bind _projectilemovement (Variables|Default|GetProjectileMovement))
  (bind _projectilemovement_2 (Variables|Default|GetProjectileMovement))
  (bind _aspaddle_bp (Utilities|Casting|CastToPaddle_BP OtherActor)
    (:then
      (CallFunction|HandleBounce (Variables|/Game/Paddle_BP.Paddle_BP_C|GetmoveDir _aspaddle_bp))
      (if (Actor|ActorHasTag OtherActor "paddle")
        (bind _outactors (Actor|GetAllActorsOfClass "/Game/InvisibleBall_BP.InvisibleBall_BP_C"))
        (Transformation|SetWorldLocation (Variables|/Script/Engine.Actor|GetRootComponent (Utilities|Array|Get(acopy) _outactors)) (Transformation|GetWorldLocation (Variables|Default|GetDefaultSceneRoot)) false false)
        (Default|CopyVelocity (Utilities|Array|Get(acopy) _outactors))
        (Variables|/Script/Engine.MovementComponent|SetVelocity _projectilemovement (Math|Vector|MakeVector (* (.X (Math|Vector|BreakVector (Variables|/Script/Engine.MovementComponent|GetVelocity _projectilemovement))) 1.25) (.Y (Math|Vector|BreakVector (Variables|/Script/Engine.MovementComponent|GetVelocity _projectilemovement))) (.Z (Math|Vector|BreakVector (Variables|/Script/Engine.MovementComponent|GetVelocity _projectilemovement)))))))
    (:CastFailed
      (bind _asenemy_paddle_bp (Utilities|Casting|CastToEnemyPaddle_BP OtherActor)
        (:then
          (CallFunction|HandleBounce (Variables|/Game/EnemyPaddle_BP.EnemyPaddle_BP_C|GetmoveDir _asenemy_paddle_bp))
          (Variables|/Script/Engine.MovementComponent|SetVelocity _projectilemovement_2 (Math|Vector|MakeVector (* (.X (Math|Vector|BreakVector (Variables|/Script/Engine.MovementComponent|GetVelocity _projectilemovement_2))) 1.25) (.Y (Math|Vector|BreakVector (Variables|/Script/Engine.MovementComponent|GetVelocity _projectilemovement_2))) (.Z (Math|Vector|BreakVector (Variables|/Script/Engine.MovementComponent|GetVelocity _projectilemovement_2))))))
        (:CastFailed
          (Utilities|Casting|CastToWall_BP OtherActor)
          (CallFunction|ReverseY))))))

(event EventTick
  (params (DeltaSeconds :type Float%20%28single-precision%29))
  (Variables|Default|SettimeSinceReversed (+ DeltaSeconds (Variables|Default|GettimeSinceReversed)))
  (bind _outofbounds (CallFunction|IsOutOfBounds))
  (if _outofbounds
    (Transformation|SetActorLocation "0, 0, 0" false false)
    (Variables|/Script/Engine.MovementComponent|SetVelocity (Variables|Default|GetProjectileMovement) (Math|Vector|MakeVector 3e+02 0.0 0.0))))

(fn ConstructionScript)

(fn IsOutOfBounds
  (bind _outactors (Actor|GetAllActorsOfClass "/Game/Paddle_BP.Paddle_BP_C"))
  (if (<= (.X (Math|Vector|BreakVector (Transformation|GetActorLocation (Utilities|Array|Get(acopy) _outactors)))) (.X (Math|Vector|BreakVector (Transformation|GetActorLocation))))
    _
    (else
      (bind _outactors_2 (Actor|GetAllActorsOfClass "/Game/EnemyPaddle_BP.EnemyPaddle_BP_C"))
      (if (>= (.X (Math|Vector|BreakVector (Transformation|GetActorLocation (Utilities|Array|Get(acopy) _outactors_2)))) (.X (Math|Vector|BreakVector (Transformation|GetActorLocation))))
        _
        (else
          (return false)))))
  (return true))

(fn HandleBounce
  (params (selection :type Integer))
  (bind _returnvalue (Math|Random|RandomFloatinRange -5e+01 5e+01))
  (switch int selection
    (:-1
      (CallFunction|AddSpin (+ _returnvalue -125.0)))
    (:0
      (CallFunction|AddSpin (Math|Random|RandomFloatinRange -15.0 15.0)))
    (:1
      (CallFunction|AddSpin (+ _returnvalue 125.0))))
  (CallFunction|ReverseX))

(fn AddSpin
  (params (spin :type Float%20%28single-precision%29))
  (Variables|/Script/Engine.MovementComponent|SetVelocity (Variables|Default|GetProjectileMovement) (+ (Math|Vector|MakeVector 0.0 spin 0.0) (Variables|/Script/Engine.MovementComponent|GetVelocity (Variables|Default|GetProjectileMovement)))))

(fn ReverseX
  (Variables|/Script/Engine.MovementComponent|SetVelocity (Variables|Default|GetProjectileMovement) (Math|Vector|MakeVector (* -1 (.X (Math|Vector|BreakVector (Variables|/Script/Engine.MovementComponent|GetVelocity (Variables|Default|GetProjectileMovement))))) (.Y (Math|Vector|BreakVector (Variables|/Script/Engine.MovementComponent|GetVelocity (Variables|Default|GetProjectileMovement)))) (.Z (Math|Vector|BreakVector (Variables|/Script/Engine.MovementComponent|GetVelocity (Variables|Default|GetProjectileMovement))))))
  (Development|PrintString "Reverse")
  (Variables|Default|SettimeSinceReversed 0.0))

(fn ReverseY
  (Variables|/Script/Engine.MovementComponent|SetVelocity (Variables|Default|GetProjectileMovement) (Math|Vector|MakeVector (.X (Math|Vector|BreakVector (Variables|/Script/Engine.MovementComponent|GetVelocity (Variables|Default|GetProjectileMovement)))) (* -1 (.Y (Math|Vector|BreakVector (Variables|/Script/Engine.MovementComponent|GetVelocity (Variables|Default|GetProjectileMovement))))) (.Z (Math|Vector|BreakVector (Variables|/Script/Engine.MovementComponent|GetVelocity (Variables|Default|GetProjectileMovement))))))
  (Development|PrintString "Reverse")
  (Variables|Default|SettimeSinceReversed 0.0))